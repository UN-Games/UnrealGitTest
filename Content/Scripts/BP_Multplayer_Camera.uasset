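; Shared multiplayer camera actor that becomes player 0's view target on BeginPlay and turns to keep the group of players in view.
; It caches all BP_Player_Move actors at BeginPlay, with G re-gathering them and printing the count.
; Each Tick (or H press) averages their capsule locations and rotates MainCamera toward that midpoint.
; The camera only rotates, with no repositioning or zoom.
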(event Collision|EventActorBeginOverlap
  (params (OtherActor :type Actor%20Object%20Reference)))

(event EventTick
  (params (DeltaSeconds :type Float%20%28single-precision%29))
  (Utilities|FlowControl|Sequence
    (:then_0
      (for _array_element (stale EventBeginPlay _outactors)
        (bind _output_get (Variables|Default|SetMeanPosition (+ (Transformation|GetWorldLocation (Variables|/Script/Engine.Character|GetCapsuleComponent _array_element)) (Variables|Default|GetMeanPosition)))))
      (bind _output_get_2 (Variables|Default|SetMeanPosition (/ _output_get (Utilities|Array|Length (stale EventBeginPlay _outactors)))))
      (Utilities|FlowControl|Sequence
        (:then_0
          (Transformation|SetWorldRotation (Variables|Default|GetMain_Camera) (Math|Rotator|FindLookatRotation (Transformation|GetWorldLocation (Variables|Default|GetMain_Camera)) _output_get_2) false false))
        (:then_1
          (Variables|Default|SetMeanPosition "0, 0, 0"))))))

(event EventBeginPlay
  (Utilities|FlowControl|Sequence
    (:then_0
      ;[1 1 1] Enable Input In this Script
      (Input|EnableInput (Game|GetPlayerController 0)))
    (:then_1
      ;[1 1 1] Set Camera On Play
      (Variables|Default|SetbFindCameraComponentWhenViewTarget true)
      (Game|Player|SetViewTargetwithBlend (Game|GetPlayerController 0) (Components|GetOwner (Variables|Default|GetMain_Camera)) 0.0 "VTBlend_Linear" 0.0 false))
    (:then_2
      ;[1 1 1] Get All Players
      (Variables|Default|SetMeanPosition "0, 0, 0")
      (bind _outactors (Actor|GetAllActorsOfClass "/Game/Scripts/BP_Player_Move.BP_Player_Move_C"))
      (Development|PrintString (Utilities|String|ToString(Integer) (Utilities|Array|Length _outactors))))))

(event Input|KeyboardEvents|G
  (params (Key :type Key%20Structure :default "None"))
  ;[1 1 1] Get All Players
  (:Pressed
    (Variables|Default|SetMeanPosition "0, 0, 0")
    (bind _outactors (Actor|GetAllActorsOfClass "/Game/Scripts/BP_Player_Move.BP_Player_Move_C"))
    (Development|PrintString (Utilities|String|ToString(Integer) (Utilities|Array|Length _outactors)))))

(event Input|KeyboardEvents|H
  (params (Key :type Key%20Structure :default "None"))
  (:Pressed
    (for _array_element (stale EventBeginPlay _outactors)
      (bind _output_get (Variables|Default|SetMeanPosition (+ (Transformation|GetWorldLocation (Variables|/Script/Engine.Character|GetCapsuleComponent _array_element)) (Variables|Default|GetMeanPosition)))))
    (bind _output_get_2 (Variables|Default|SetMeanPosition (/ _output_get (Utilities|Array|Length (stale EventBeginPlay _outactors)))))
    (Utilities|FlowControl|Sequence
      (:then_0
        (Transformation|SetWorldRotation (Variables|Default|GetMain_Camera) (Math|Rotator|FindLookatRotation (Transformation|GetWorldLocation (Variables|Default|GetMain_Camera)) _output_get_2) false false))
      (:then_1
        (Variables|Default|SetMeanPosition "0, 0, 0")))))

(fn ConstructionScript)